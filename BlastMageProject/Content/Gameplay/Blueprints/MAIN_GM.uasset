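; MAIN_GM is a game mode Blueprint that spawns and sets up local multiplayer characters at BeginPlay.
; It gathers all PlayerStarts, then matches each player index up to PlayerCount to the start tagged "P" plus that index.
; For each match it creates a local player, spawns and possesses a PLAYER_CHARACTER, records it in Players, tags it with a one-based PLAYER_ name and sets the controller ID.
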(event `self.ReceiveBeginPlay`
  (`self.Get Player Start Points`)
  (`self.Spawn Players`))

(fn `Get Player Start Points`
  (bind _outactors (`GameplayStatics.GetAllActorsOfClass` "/Script/Engine.PlayerStart"))
  (set `self.Player Starts` _outactors))

(fn `Spawn Players`
  (bind _returnvalue (`GameplayStatics.GetPlayerController` (`self.Index`)))
  (for _index (range (`self.Player Count`))
    (set `self.Index` _index)
    (for _array_element (`self.Player Starts`)
      (if (== (`PlayerStart.PlayerStartTag` _array_element) (`KismetStringLibrary.Conv_StringToName` (`KismetStringLibrary.Concat_StrStr` "P" (`KismetStringLibrary.Conv_IntToString` (`self.Index`)))))
        (`GameplayStatics.CreatePlayer` (`self.Index`))
        (bind _returnvalue_2 (`|SpawnActorFromClass` "/Game/Gameplay/Blueprints/PLAYER_CHARACTER.PLAYER_CHARACTER_C" (`self.GetTransform` _array_element) "AlwaysSpawn" "OverrideRootScale" null (`self.Index`) null))
        (`Controller.Possess` _returnvalue _returnvalue_2)
        (`KismetArrayLibrary.Array_AddUnique` (`self.Players`) _returnvalue_2)
        (set `Actor.Tags` (`|MakeArray` (`KismetStringLibrary.Conv_StringToName` (`KismetStringLibrary.Concat_StrStr` "PLAYER_" (`KismetStringLibrary.Conv_IntToString` (+ (`self.Index`) 1))))) _returnvalue_2)
        (`GameplayStatics.SetPlayerControllerID` _returnvalue (`self.Index`))))))

(fn `UserConstructionScript`)