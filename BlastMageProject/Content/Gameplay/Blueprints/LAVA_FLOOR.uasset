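; LAVA_FLOOR is a lava hazard that damages and knocks back any PLAYER_CHARACTER touching it.
; The collider's begin-overlap applies damage, then knockback and a 2D step sound if the player is still valid.
; As a fallback for missed re-touches, Tick scans overlapping actors and, after a short delay, repeats damage and knockback without sound if the player still overlaps.
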(event `self.ReceiveTick`
  (params (DeltaSeconds :type "Float (single-precision)"))
  ;[1 1 1] If, for some reason, the engine does not read that the player has stopped touching the lava and retouched it, check if they're touching it for too long.
  (for _array_element (`self.GetOverlappingActors` null)
    (bind _asplayer_character (cast `/Game/Gameplay/Blueprints/PLAYER_CHARACTER` _array_element))
    (`KismetSystemLibrary.Delay` 0.15)
    (if (`self.IsOverlappingActor` _asplayer_character)
      (`/Game/Gameplay/Blueprints/PLAYER_CHARACTER.TakeDamage` _asplayer_character (`self.Damage`))
      (`/Engine/EditorBlueprintResources/StandardMacros.IsValid` _asplayer_character ; To make sure we don't try to apply knockback to a dead player
        (:`Is Valid`
          (`/Game/Gameplay/Blueprints/PLAYER_CHARACTER.Take Knockback` _asplayer_character (`self.Knockback`)))))))

(event `self.Collider.OnComponentBeginOverlap`
  (params (OverlappedComponent :type "PrimitiveComponent Object Reference") (OtherActor :type "Actor Object Reference") (OtherComp :type "PrimitiveComponent Object Reference") (OtherBodyIndex :type Integer) (bFromSweep :type Boolean) (SweepResult :type "HitResult Structure (by ref)"))
  ;[1 1 1] The player manually touches the lava
  (bind _asplayer_character (cast `/Game/Gameplay/Blueprints/PLAYER_CHARACTER` OtherActor))
  (`/Game/Gameplay/Blueprints/PLAYER_CHARACTER.TakeDamage` _asplayer_character (`self.Damage`))
  (`/Engine/EditorBlueprintResources/StandardMacros.IsValid` _asplayer_character ; To make sure we don't try to apply knockback to a dead player
    (:`Is Valid`
      (`/Game/Gameplay/Blueprints/PLAYER_CHARACTER.Take Knockback` _asplayer_character (`self.Knockback`))
      (`GameplayStatics.PlaySound2D` "/Game/SoundEffect/lavastepon.lavastepon" 1.0 1.0 0.0 null null))))

(fn `UserConstructionScript`)