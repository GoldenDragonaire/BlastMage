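; Spawner actor that periodically creates Item_ShieldPotion pickups in the level.
; BeginPlay starts a looping timer whose interval is ItemDelay randomly offset within a SpawnVarience range, rolled once per instance.
; Each tick of the timer calls SpawnItem, which spawns the potion at ShootOffset rotated into the actor's orientation, with the actor's rotation.
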(event `self.ReceiveBeginPlay`
  (bind _spawn_varience (`self.Spawn Varience`))
  (`KismetSystemLibrary.K2_SetTimerDelegate` (delegate `SpawnShield`) (+ (`self.ItemDelay`) (- (* (`KismetMathLibrary.RandomFloat`) _spawn_varience) (* _spawn_varience 0.5))) true))

(event `SpawnShield`
  (`self.SpawnItem`))

(fn `SpawnItem`
  (bind _returnvalue (`self.K2_GetActorRotation`))
  (`|SpawnActorFromClass` "/Game/Blueprints/Items/Item_ShieldPotion.Item_ShieldPotion_C" (`KismetMathLibrary.MakeTransform` (+ (`self.K2_GetActorLocation`) (`KismetMathLibrary.GreaterGreater_VectorRotator` (`self.ShootOffset`) _returnvalue)) _returnvalue) "Undefined" "OverrideRootScale" null null))

(fn `UserConstructionScript`)