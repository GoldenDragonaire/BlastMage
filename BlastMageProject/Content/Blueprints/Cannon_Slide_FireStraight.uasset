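; Cannon actor that slides along a horizontal offset from its start point while firing fireballs straight ahead on a looping timer.
; Tick drives a timeline that lerps a swept move between start and slide target, replaying in its current direction on finish.
; The timer calls CannonShoot, which spawns the projectile at a rotated offset, applies GetCannonBall's speed, damage and knockback, then plays a fire sound.
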(event `Shoot Cannon`
  ;[1 1 1] Shoot Cannon
  (`self.Cannon Shoot`))

(event `self.ReceiveTick`
  (params (DeltaSeconds :type "Float (single-precision)"))
  ;[1 1 1] Cannon Smooth Slide
  (bind (_direction _newtrack_0) (`Timeline|MoveTimeline` :!label _label)
    (:`Update`
      (bind _output_get (set `self.targetLocation` (`KismetMathLibrary.VLerp` (stale `self.ReceiveBeginPlay` _output_get) (`KismetMathLibrary.MakeVector` (+ (`self.SlideDistanceX`) (.x (stale `self.ReceiveBeginPlay` _output_get))) (+ (.y (stale `self.ReceiveBeginPlay` _output_get)) (`self.SlideDistanceY`)) (.z (stale `self.ReceiveBeginPlay` _output_get))) _newtrack_0)))
      (`self.K2_SetActorLocation` _output_get true))
    (:`Finished`
      (switch `ETimelineDirection` _direction
        (:`Forward`
          (goto _label :!via `PlayFromStart`))
        (:`Backward`
          (goto _label :!via `ReverseFromEnd`))))))

(event `self.ReceiveBeginPlay`
  ;[1 1 1] Cannon Smooth Slide
  (bind _output_get (set `self.initLocation` (`self.K2_GetActorLocation`)))
  ;[1 1 1] Shoot Cannon
  (`KismetSystemLibrary.K2_SetTimerDelegate` (delegate `Shoot Cannon`) (`self.FireRate`) true))

(fn `Cannon Shoot`
  (bind _returnvalue (`self.K2_GetActorRotation`))
  (bind _returnvalue_2 (+ (`self.K2_GetActorLocation`) (`KismetMathLibrary.GreaterGreater_VectorRotator` (`self.ShootOffset`) _returnvalue)))
  (bind (_projectile_class _speed _damage _knockback_scale _fire_sound) (`self.GetCannonBall`))
  ;[1 1 1] Spawn Projectile at location
  (bind _returnvalue_3 (`|SpawnActorFromClass` _projectile_class (`KismetMathLibrary.MakeTransform` _returnvalue_2 _returnvalue) "AdjustIfPossibleButAlwaysSpawn" "OverrideRootScale" null null))
  (`/Engine/EditorBlueprintResources/StandardMacros.IsValid` _returnvalue_3
    (:`Is Valid`
      (`/Game/Gameplay/Blueprints/PROJECTILE_BP/PROJ_BASE.Set Speed` _returnvalue_3 _speed)
      (`/Game/Gameplay/Blueprints/PROJECTILE_BP/PROJ_BASE.Set Damage` _returnvalue_3 _damage)
      (`/Game/Gameplay/Blueprints/PROJECTILE_BP/PROJ_BASE.Set Knockback` _returnvalue_3 _knockback_scale)
      (`GameplayStatics.PlaySoundAtLocation` _fire_sound _returnvalue_2 (struct) 1.0 1.0 0.0 null null null))))

(fn `GetCannonBall`
  (returns (`Projectile Class` :type "/Game/Gameplay/Blueprints/PROJECTILE_BP/PROJ_BASE Class Reference") (Speed :type "Float (double-precision)") (Damage :type "Float (double-precision)") (`Knockback Scale` :type "Float (double-precision)") (`Fire Sound` :type "SoundBase Object Reference"))
  (return "/Game/Gameplay/Blueprints/PROJECTILE_BP/PROJ_FIREBALL.PROJ_FIREBALL_C" 1000.0 20.0 400.0 null))

(fn `UserConstructionScript`)