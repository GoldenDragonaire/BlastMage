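; FloorTile is a floor piece that drops away over time, so tiles farther from the world origin fall earlier.
; Tick compares time since the tile's creation to a two-minute limit, shortened in proportion to its horizontal distance from the origin.
; Once past it, a Fall flag starts a timeline once, whose updates lower the tile by a fixed step, making fall speed frame-rate dependent.
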(event `self.ReceiveTick`
  (params (DeltaSeconds :type "Float (single-precision)"))
  (bind _x (.x (`self.K2_GetActorLocation`)))
  (bind _y (.y (`self.K2_GetActorLocation`)))
  (if (> (`self.GetGameTimeSinceCreation`) (- 120.0 (/ (`KismetMathLibrary.Sqrt` (+ (`KismetMathLibrary.Square` _x) (`KismetMathLibrary.Square` _y))) 10.0)))
    (if (not (`self.fall`))
      (set `self.fall` true)
      (`Timeline|fall_timeline`
        (:`Update`
          (`self.K2_SetActorLocation` (+ (`KismetMathLibrary.MakeVector` _x _y (.z (`self.K2_GetActorLocation`))) (0.0 0.0 -0.25))))))))

(fn `UserConstructionScript`)