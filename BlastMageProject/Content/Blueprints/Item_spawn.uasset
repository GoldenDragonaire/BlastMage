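; Item spawner actor that periodically spawns a random item class from its item list.
; On BeginPlay it starts a looping timer, with the interval randomized once around ItemDelay by SpawnVarience.
; Each tick of that timer swaps the Plane to a glow material for a short warning delay, switches to another glow material, then spawns the item at a rotation-relative offset from the actor.
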(event `self.ReceiveBeginPlay`
  (bind _spawn_varience (`self.Spawn Varience`))
  (`KismetSystemLibrary.K2_SetTimerDelegate` (delegate `SpawnShield`) (+ (`self.ItemDelay`) (- (* (`KismetMathLibrary.RandomFloat`) _spawn_varience) (* _spawn_varience 0.5))) true))

(event `SpawnShield`
  (`PrimitiveComponent.SetMaterial` (`self.Plane`) 0 "/Game/ModularMagicCircles/Materials/MI_Fade+Glow_01.MI_Fade+Glow_01")
  (`KismetSystemLibrary.Delay` 3.0)
  (`PrimitiveComponent.SetMaterial` (`self.Plane`) 0 "/Game/ModularMagicCircles/Materials/MI_Fade+Glow_03.MI_Fade+Glow_03")
  (`self.SpawnItem`))

(fn `SpawnItem`
  (bind _returnvalue (`self.K2_GetActorRotation`))
  (bind _itemlist (`self.itemList`))
  (`|SpawnActorFromClass` (`|GetArrayItem` _itemlist (`KismetMathLibrary.RandomInteger` (`KismetArrayLibrary.Array_Length` _itemlist))) (`KismetMathLibrary.MakeTransform` (+ (`self.K2_GetActorLocation`) (`KismetMathLibrary.GreaterGreater_VectorRotator` (`self.ShootOffset`) _returnvalue)) _returnvalue) "Undefined" "OverrideRootScale" null null))

(fn `UserConstructionScript`)